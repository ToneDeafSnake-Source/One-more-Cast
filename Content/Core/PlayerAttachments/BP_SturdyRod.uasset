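; BP_SturdyRod is a player attachment Blueprint for a sturdy rod, apparently for fishing, that switches the rod mesh between preset poses.
; Three custom events set the relative rotation of BasicRodMesh to default, idle-correction or catch-correction rotation variables.
; The events are not called within this graph, and the construction script and standard lifecycle events are empty.
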(event `ApplyRodDefaultPose`
  (`SceneComponent.K2_SetRelativeRotation` (`self.BasicRodMesh`) (`self.RodDefaultRotation`) false false))

(event `ApplyRodCorrectionPose`
  (`SceneComponent.K2_SetRelativeRotation` (`self.BasicRodMesh`) (`self.RodIdleCorrection`) false false))

(event `ApplyRodCatchCorrectionPose`
  (`SceneComponent.K2_SetRelativeRotation` (`self.BasicRodMesh`) (`self.RodCatchCorrection`) false false))

(fn `UserConstructionScript`)