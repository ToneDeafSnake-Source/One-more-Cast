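; BP_FishingSpot is an interactable spot where BP_Fisherman casts, waits for a random bite and catches fish, junk or treasure.
; It registers with the focused fisherman, checks pass tier and inventory space, then drives animations, rod poses and status messages through each stage.
; Catches roll species by explicit odds or weighted fallback, then quality, weight and value.
; Rare and legendary catches open a roll popup; others go straight to inventory.
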(event `/Game/Core/UI_Components/BPI_Interact.SetInteractionFocused`
  (params (IsFocused :type Boolean) (InteractingPlayer :type "Character Object Reference"))
  ;[0.15 0.15 0.15 0.5 40] Determines if player is close enough to the fishing spot
  (if IsFocused
    (bind _asbp_fisherman (cast `/Game/Core/PlayerBlueprints/BP_Fisherman` InteractingPlayer))
    (`/Game/Core/PlayerBlueprints/BP_Fisherman.RegisterFishingSpot` _asbp_fisherman self)
    (else
      (bind _asbp_fisherman_2 (cast `/Game/Core/PlayerBlueprints/BP_Fisherman` InteractingPlayer))
      (`/Game/Core/PlayerBlueprints/BP_Fisherman.UnregisterFishingSpot` _asbp_fisherman_2 self))))

(event `/Game/Core/UI_Components/BPI_Interact.OnInteract`
  (params (InteractingPlayer :type "Character Object Reference"))
  ;[0.15 0.15 0.15 0.5 40] Catching Fish
  (bind _asbp_fisherman (cast `/Game/Core/PlayerBlueprints/BP_Fisherman` InteractingPlayer))
  (bind _output_get (set `self.ActiveFisherman` _asbp_fisherman))
  (if (`/Game/Core/PlayerBlueprints/BP_Fisherman.CanPlayerFish` _output_get)
    (`/Game/Core/PlayerBlueprints/BP_Fisherman.MoveIntoFishingPosition` _output_get self)
    (if (`KismetSystemLibrary.IsValid` (`/Game/Core/PlayerBlueprints/BP_Fisherman.StartFishingWidget` _output_get))
      (`/Game/Core/PlayerBlueprints/BP_Fisherman.HideStartFishingWidget` (`self.ActiveFisherman`)))))

(event `BeginFishingAfterPositioned`
  (params (`Interacting Player` :type "Character Object Reference"))
  (bind _activefisherman (`self.ActiveFisherman`))
  ;[0.15 0.15 0.15 0.5 40] Catching Fish
  (bind _asbp_fisherman (cast `/Game/Core/PlayerBlueprints/BP_Fisherman` `Interacting Player`))
  (bind _output_get (set `self.ActiveFisherman` _asbp_fisherman))
  (if (`KismetSystemLibrary.IsValid` _output_get)
    (if (== (`/Game/Core/PlayerBlueprints/BP_Fisherman.CurrentFishingSpot` (`self.ActiveFisherman`)) self)
      (if (not (`/Game/Core/PlayerBlueprints/BP_Fisherman.bFishingRollPopupOpen` _output_get))
        (`self.CheckFishingPassLevel` (`/Game/Core/PlayerBlueprints/BP_Fisherman.FishingPassTier` _output_get) (`self.RequiredPassTier`))
        (if (`self.CorrectFishingPass`)
          (bind _has_room (`/Game/Core/Inventory_Systems/BP_InventoryComponent.Has room` (`/Game/Core/PlayerBlueprints/BP_Fisherman.BP_InventoryComponent` _asbp_fisherman)))
          (if _has_room
            (if (`/Game/Core/PlayerBlueprints/BP_Fisherman.CanPlayerFish` _output_get)
              (bind _startfishingwidget (`/Game/Core/PlayerBlueprints/BP_Fisherman.StartFishingWidget` _output_get))
              (if (`KismetSystemLibrary.IsValid` _startfishingwidget)
                (`Widget.RemoveFromParent` _startfishingwidget))
              (if (`/Game/Core/PlayerBlueprints/BP_Fisherman.IsFishing` _output_get)
                (`/Game/Core/PlayerBlueprints/BP_Fisherman.ShowSecondaryStatus` _output_get (`self.AlreadyFishingMessage`))
                (else
                  (set `/Game/Core/PlayerBlueprints/BP_Fisherman.IsFishing` true _output_get)
                  (`CharacterMovementComponent.DisableMovement` (`Character.CharacterMovement` _output_get))
                  (set `/Game/Core/PlayerBlueprints/BP_Fisherman.CurrentFishingSpot` self _output_get)
                  (`/Game/Core/PlayerBlueprints/BP_Fisherman.ShowFishingStatus` _activefisherman (`self.CastingMessage`))
                  (`/Game/Core/PlayerBlueprints/BP_Fisherman.EquipFishingRod` _activefisherman)
                  (`/Game/Core/PlayerBlueprints/BP_Fisherman.ApplyRodDefaultPose` _activefisherman)
                  (set `/Game/Core/PlayerBlueprints/BP_Fisherman.bUseFishingLeftHandIK` false _activefisherman)
                  (`/Game/Core/PlayerBlueprints/BP_Fisherman.PlayFishingCastAnimation` _activefisherman))))
            (else
              (`CharacterMovementComponent.SetMovementMode` (`Character.CharacterMovement` _output_get) "MOVE_Walking" 0)
              (if (not (`KismetSystemLibrary.IsValid` (`/Game/Core/PlayerBlueprints/BP_Fisherman.FishingStatusWidget` _output_get)))
                (`/Game/Core/PlayerBlueprints/BP_Fisherman.ShowFishingStatus` _output_get (`self.InventoryFullMessage`))
                (`KismetSystemLibrary.Delay` 2.0)
                (if (`KismetSystemLibrary.IsValid` (`/Game/Core/PlayerBlueprints/BP_Fisherman.FishingStatusWidget` _output_get))
                  (`/Game/Core/PlayerBlueprints/BP_Fisherman.HideFishingStatus` _output_get))))))))))

(event `ContinueAfterCasting`
  (bind _activefisherman (`self.ActiveFisherman`))
  (bind _activefisherman_2 (`self.ActiveFisherman`))
  ;[0.15 0.15 0.15 0.5 40] Catching Fish
  (`/Game/Core/PlayerBlueprints/BP_Fisherman.ShowFishingStatus` _activefisherman_2 (`self.WaitingMessage`))
  (`/Game/Core/PlayerBlueprints/BP_Fisherman.ApplyRodCastCorrection` _activefisherman_2)
  (`/Game/Core/PlayerBlueprints/BP_Fisherman.PlayIdleFishingAnimation` _activefisherman_2)
  (set `/Game/Core/PlayerBlueprints/BP_Fisherman.bUseFishingLeftHandIK` true _activefisherman_2)
  (set `/Game/Core/PlayerBlueprints/BP_Fisherman.bUseFishingRightHandIK` true _activefisherman_2)
  (`KismetSystemLibrary.Delay` (`KismetMathLibrary.RandomFloatInRange` (`self.MinBiteTime`) (`self.MaxBiteTime`)))
  (if (`/Game/Core/PlayerBlueprints/BP_Fisherman.IsFishing` _activefisherman_2)
    (`/Game/Core/PlayerBlueprints/BP_Fisherman.ShowFishingStatus` _activefisherman (`self.BiteMessage`))
    (`/Game/Core/PlayerBlueprints/BP_Fisherman.ApplyRodCatchCorrection` _activefisherman)
    (set `/Game/Core/PlayerBlueprints/BP_Fisherman.bUseFishingLeftHandIK` true _activefisherman)
    (`/Game/Core/PlayerBlueprints/BP_Fisherman.PlayCatchingAnimation` _activefisherman)))

(event `FinishCatch`
  (bind _activefisherman (`self.ActiveFisherman`))
  (bind _activefisherman_2 (`self.ActiveFisherman`))
  ;[0.15 0.15 0.15 0.5 40] Catching Fish
  (`self.ChoosingFishToCatch`)
  (`/Game/Core/PlayerBlueprints/BP_Fisherman.HideFishingStatus` _activefisherman)
  (set `/Game/Core/PlayerBlueprints/BP_Fisherman.IsFishing` false _activefisherman)
  (`CharacterMovementComponent.SetMovementMode` (`Character.CharacterMovement` _activefisherman) "MOVE_Walking" 0)
  (`/Game/Core/PlayerBlueprints/BP_Fisherman.UnequipFishingRod` _activefisherman_2)
  (`/Game/Core/PlayerBlueprints/BP_Fisherman.ApplyRodDefaultPose` _activefisherman_2)
  (set `/Game/Core/PlayerBlueprints/BP_Fisherman.bUseFishingLeftHandIK` false _activefisherman_2)
  (if (not (`/Game/Core/PlayerBlueprints/BP_Fisherman.bFishingRollPopupOpen` _activefisherman_2))
    (`/Game/Core/PlayerBlueprints/BP_Fisherman.ShowStartFishingWidget` _activefisherman_2)))

(fn `BuildCaughtFishItem`
  (params (SelectedQuality :type "/Game/Core/Data/Structs/ST_FishQualityEntry Structure") (SelectedFish :type "/Game/Core/Data/Structs/ST_FishCatchEntry Structure"))
  (returns (CaughtItem :type "/Game/Core/Data/Structs/ST_ItemData Structure"))
  (locals (FinalWeight :type "Float (double-precision)" :default 0.0) (FinalSellValue :type Integer :default 0) (FinalDisplayName :type Text) (Local_ReqCatchDC :type Integer) (Local_IsRare :type Boolean) (Local_IsLegendary :type Boolean) (Local_Quality :type "/Game/Core/Data/Enum/E_FishQuality Enum") (Local_ValueMultiplier :type "Float (double-precision)") (Local_MaxWeight :type "Float (double-precision)") (Local_MinWeight :type "Float (double-precision)"))
  (bind (_fishid _fishdisplayname _fishicon _basesellvalue _explicitcatchratedenominator _commonrollweighting _qualitytable _buseexplicitcatchrate _bisfishcatch _bisjunkcatch _bistreasurecatch) (break `/Game/Core/Data/Structs/ST_FishCatchEntry` SelectedFish))
  (bind (_quality _ratedenominator _valuemultiplier _minweight _maxweight _requiredcatchdc) (break `/Game/Core/Data/Structs/ST_FishQualityEntry` SelectedQuality))
  (set `local.Local_MinWeight` _minweight)
  (set `local.Local_MaxWeight` _maxweight)
  (set `local.Local_ValueMultiplier` _valuemultiplier)
  (set `local.Local_ReqCatchDC` _requiredcatchdc)
  (set `local.Local_Quality` _quality)
  (set `local.Local_IsRare` (`|EnumEquality` _quality "NewEnumerator1"))
  (set `local.Local_IsLegendary` (`|EnumEquality` _quality "NewEnumerator0"))
  (set `local.FinalWeight` (`KismetMathLibrary.RandomFloatInRange` (`local.Local_MinWeight`) (`local.Local_MaxWeight`)))
  (set `local.FinalSellValue` (`KismetMathLibrary.Round` (* (`KismetMathLibrary.Conv_IntToDouble` _basesellvalue) (`local.Local_ValueMultiplier`))))
  (bind (_resolvedname _resolvedicon) (`self.ResolveCatchPresentation` _fishid _fishdisplayname _fishicon))
  (set `local.FinalDisplayName` (`|FormatText` "{prefix} {FishName}" (`|GenericToText` (`local.Local_Quality`)) _resolvedname))
  (return (make `/Game/Core/Data/Structs/ST_ItemData` (`KismetTextLibrary.Conv_TextToString` (`local.FinalDisplayName`)) (`local.FinalDisplayName`) 1 (`local.Local_ReqCatchDC`) (`local.FinalSellValue`) _resolvedicon 0.0 0.0 (`local.FinalWeight`) _fishid _fishid (`local.Local_Quality`) (`local.Local_IsLegendary`) (`local.Local_IsRare`) _bisfishcatch true _bisjunkcatch _bistreasurecatch)))

(fn `CheckFishingPassLevel`
  (params (PlayerPassLevel :type Integer) (RequiredPassTier :type Integer))
  (`KismetSystemLibrary.PrintString` (`KismetStringLibrary.Conv_IntToString` PlayerPassLevel))
  (if (>= PlayerPassLevel RequiredPassTier)
    (set `self.CorrectFishingPass` true)
    (return)
    (else
      (`KismetSystemLibrary.PrintString` "You may have skipped the gate. But you can't fish here until you have the pass"))))

(fn `ChoosingFishToCatch`
  (locals (RolledWeight :type "Float (double-precision)") (WeightPercent :type "Float (double-precision)") (`Final Sell Value` :type Integer) (BaseSellValue :type Integer) (D20Roll :type Integer) (FinalRoll :type Integer) (RequiredRoll :type Integer) (BP_Fisherman :type "/Game/Core/PlayerBlueprints/BP_Fisherman Object Reference"))
  (bind _returnvalue (`GameplayStatics.GetPlayerController` 0))
  ; What fish is being caught?
  (if (> (`KismetArrayLibrary.Array_Length` (`self.FishCatchTable`)) 0)
    (bind (_bfoundfish _selectedfish) (`self.RollFishSpecies`))
    (if _bfoundfish
      (bind (_bfoundquality _selectedquality) (`self.RollFishQuality` _selectedfish))
      (if _bfoundquality
        (bind _caughtitem (`self.BuildCaughtFishItem` _selectedquality _selectedfish))
        (bind _output_get (set `self.CaughtFish` _caughtitem))
        (bind (_itemname _basename _quantity _catchdc _sellvalue _itemicon _minweight _maxweight _fishweight _itemid _fishid _quality _islegendaryfish _israrefish) (break `/Game/Core/Data/Structs/ST_ItemData` _output_get))
        (if (or _islegendaryfish _israrefish)
          (bind _asbp_fisherman (cast `/Game/Core/PlayerBlueprints/BP_Fisherman` (`GameplayStatics.GetPlayerCharacter` 0)))
          (bind _inventorywidget (`/Game/Core/PlayerBlueprints/BP_Fisherman.InventoryWidget` _asbp_fisherman))
          (if (`KismetSystemLibrary.IsValid` _inventorywidget)
            (`Widget.RemoveFromParent` _inventorywidget)
            (set `/Game/Core/PlayerBlueprints/BP_Fisherman.InventoryWidget` null _asbp_fisherman))
          (bind _returnvalue_2 (`|CreateWidget` "/Game/Core/UI_Components/Menus/FishingRollPopup/WBP_FishingRollPopup.WBP_FishingRollPopup_C" null _catchdc (`/Game/Core/PlayerBlueprints/BP_Fisherman.BaseCatchBonus` _asbp_fisherman) _asbp_fisherman (make `/Game/Core/Data/Structs/ST_FishingRollContext` (`self.CaughtFish`) self)))
          (`/Game/Core/PlayerBlueprints/BP_Fisherman.ClearActiveRollBaits` _asbp_fisherman)
          (`UserWidget.AddToViewport` _returnvalue_2 0)
          (set `/Game/Core/PlayerBlueprints/BP_Fisherman.bFishingRollPopupOpen` true _asbp_fisherman)
          (set `PlayerController.bShowMouseCursor` true _returnvalue)
          (`WidgetBlueprintLibrary.SetInputMode_UIOnlyEx` _returnvalue _returnvalue_2)
          (else
            (bind _asbp_fisherman_2 (cast `/Game/Core/PlayerBlueprints/BP_Fisherman` (`GameplayStatics.GetPlayerCharacter` 0)))
            (`/Game/Core/PlayerBlueprints/BP_Fisherman.AddCaughtFishToInventory` _asbp_fisherman_2 _output_get)
            (`/Game/Core/PlayerBlueprints/BP_Fisherman.UnequipFishingRod` _asbp_fisherman_2)
            (`/Game/Core/PlayerBlueprints/BP_Fisherman.ShowStartFishingWidget` _asbp_fisherman_2)
            (return)))
        (else
          (`KismetSystemLibrary.PrintString` "No fish quality found")))
      (else
        (`KismetSystemLibrary.PrintString` "No fish spieces Found")))
    (else
      (`KismetSystemLibrary.PrintString` "FishCatchTable is empty"))))

(fn `IsInteractable`
  (returns (Interactable :type Boolean))
  (return false))

(fn `ResolveCatchPresentation`
  (params (FishID :type Name) (FallbackName :type Text) (FallBackIcon :type "Texture2D Object Reference"))
  (returns (ResolvedName :type Text) (ResolvedIcon :type "Texture2D Object Reference"))
  (bind _returnvalue (`|GetDataTableRow` "/Game/Core/Data/DataTables/CollectionLog/DT_CatchDefinitions.DT_CatchDefinitions" FishID)
    (:`then`
      (bind (_displayname _icon) (break `/Game/Core/Data/Structs/CollectionLog/ST_CatchDefinition` _returnvalue))
      (return _displayname _icon))
    (:`RowNotFound`
      (return FallbackName FallBackIcon))))

(fn `RollFishQuality`
  (params (SelectedFish :type "/Game/Core/Data/Structs/ST_FishCatchEntry Structure"))
  (returns (bFoundQuality :type Boolean) (SelectedQuality :type "/Game/Core/Data/Structs/ST_FishQualityEntry Structure"))
  (bind (_fishid _fishdisplayname _fishicon _basesellvalue _explicitcatchratedenominator _commonrollweighting _qualitytable) (break `/Game/Core/Data/Structs/ST_FishCatchEntry` SelectedFish))
  (for _array_element _qualitytable
    (bind (_quality _ratedenominator) (break `/Game/Core/Data/Structs/ST_FishQualityEntry` _array_element))
    (if (and (`|EnumInequality` _quality "NewEnumerator4") (> _ratedenominator 0))
      (if (== (`KismetMathLibrary.RandomIntegerInRange` 1 _ratedenominator) 1)
        (return true _array_element))))
  (for _array_element_2 _qualitytable
    (if (`|EnumEquality` (`.Quality_2_9730D5F541FB8F17D9D897B40FB5D3EA` (break `/Game/Core/Data/Structs/ST_FishQualityEntry` _array_element_2)) "NewEnumerator4")
      (return true _array_element_2)))
  (if (> (`KismetArrayLibrary.Array_Length` _qualitytable) 0)
    (return true (`|GetArrayItem` _qualitytable))
    (else
      (`KismetSystemLibrary.PrintString` "Fish has no quality entries")
      (return false))))

(fn `RollFishSpecies`
  (returns (bFoundFish :type Boolean) (SelectedFish :type "/Game/Core/Data/Structs/ST_FishCatchEntry Structure"))
  (locals (TotalCommonWeighting :type Integer) (RollValue :type Integer) (RunningWeighting :type Integer))
  (bind _runningweighting (`local.RunningWeighting`))
  (for _array_element (`self.FishCatchTable`)
    (bind (_fishid _fishdisplayname _fishicon _basesellvalue _explicitcatchratedenominator _commonrollweighting _qualitytable _buseexplicitcatchrate) (break `/Game/Core/Data/Structs/ST_FishCatchEntry` _array_element))
    (if (and _buseexplicitcatchrate (> _explicitcatchratedenominator 0))
      (if (== (`KismetMathLibrary.RandomIntegerInRange` 1 _explicitcatchratedenominator) 1)
        (return true _array_element))))
  (set `local.TotalCommonWeighting` 0)
  (for _array_element_2 (`self.FishCatchTable`)
    (bind (_fishid_2 _fishdisplayname_2 _fishicon_2 _basesellvalue_2 _explicitcatchratedenominator_2 _commonrollweighting_2 _qualitytable_2 _buseexplicitcatchrate_2) (break `/Game/Core/Data/Structs/ST_FishCatchEntry` _array_element_2))
    (if (== (not _buseexplicitcatchrate_2) (> _commonrollweighting_2 0))
      (set `local.TotalCommonWeighting` (+ _commonrollweighting_2 (`local.TotalCommonWeighting`)))))
  (if (> (`local.TotalCommonWeighting`) 0)
    (set `local.RollValue` (`KismetMathLibrary.RandomIntegerInRange` 0 (`local.TotalCommonWeighting`)))
    (set `local.RunningWeighting` 0)
    (for _array_element_3 (`self.FishCatchTable`)
      (bind (_fishid_3 _fishdisplayname_3 _fishicon_3 _basesellvalue_3 _explicitcatchratedenominator_3 _commonrollweighting_3 _qualitytable_3 _buseexplicitcatchrate_3) (break `/Game/Core/Data/Structs/ST_FishCatchEntry` _array_element_3))
      (if (and (== _buseexplicitcatchrate_3 false) (> _commonrollweighting_3 0))
        (set `local.RunningWeighting` (+ _commonrollweighting_3 _runningweighting))
        (if (<= (`local.RollValue`) _runningweighting)
          (return true _array_element_3))))
    (else
      (`KismetSystemLibrary.PrintString` "No Valid Common Fish in Table")
      (return false))))

(fn `UserConstructionScript`)