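; Pier access gate that lets a fisherman through only with a high enough fishing pass tier.
; Overlapping AccessTrigger compares the pass to RequiredPassTier, then either permanently opens the gate by disabling BlockerCollision or prints DeniedMessage and keeps it blocking.
; The fisherman records checked piers by PierID, so ApprovedMessage prints only on the first approval.
; Feedback uses PrintString only.
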(event `self.AccessTrigger.OnComponentBeginOverlap`
  (params (OverlappedComponent :type "PrimitiveComponent Object Reference") (OtherActor :type "Actor Object Reference") (OtherComp :type "PrimitiveComponent Object Reference") (OtherBodyIndex :type Integer) (bFromSweep :type Boolean) (SweepResult :type "HitResult Structure (by ref)"))
  (bind _asbp_fisherman (cast `/Game/ThirdPerson/Blueprints/Player_Blueprints/BP_Fisherman` OtherActor))
  (if (`self.bGateOpen`)
    _
    (elif (>= (`/Game/ThirdPerson/Blueprints/Player_Blueprints/BP_Fisherman.FishingPassTier` _asbp_fisherman) (`self.RequiredPassTier`))
      (bind _hasbeenchecked (`/Game/ThirdPerson/Blueprints/Player_Blueprints/BP_Fisherman.HasPierBeenChecked` _asbp_fisherman (`self.PierID`)))
      (if _hasbeenchecked
        (set `self.bGateOpen` true)
        (`PrimitiveComponent.SetCollisionEnabled` (`self.BlockerCollision`) "NoCollision")
        (else
          (`/Game/ThirdPerson/Blueprints/Player_Blueprints/BP_Fisherman.MarkPierChecked` _asbp_fisherman (`self.PierID`))
          (`KismetSystemLibrary.PrintString` (`KismetTextLibrary.Conv_TextToString` (`self.ApprovedMessage`)))
          (set `self.bGateOpen` true)
          (`PrimitiveComponent.SetCollisionEnabled` (`self.BlockerCollision`) "NoCollision")))
      (else
        (`KismetSystemLibrary.PrintString` (`KismetTextLibrary.Conv_TextToString` (`self.DeniedMessage`)))
        (`PrimitiveComponent.SetCollisionEnabled` (`self.BlockerCollision`) "QueryAndPhysics")))))

(fn `UserConstructionScript`)