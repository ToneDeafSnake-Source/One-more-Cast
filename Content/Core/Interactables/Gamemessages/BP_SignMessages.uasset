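; BP_SignMessages is an interactable sign that shows a popup message to the fisherman player.
; Gaining focus enables interaction and shows the InteractWidget prompt; interacting creates a single WBP_SignMessage with its configured text and FishToDisplay, then hides the prompt.
; Losing focus disables interaction, hides the prompt and removes the active message.
; Overlap events are empty, and IsInteractable always returns false.
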(event `self.OverlapTrigger.OnComponentBeginOverlap`
  (params (OverlappedComponent :type "PrimitiveComponent Object Reference") (OtherActor :type "Actor Object Reference") (OtherComp :type "PrimitiveComponent Object Reference") (OtherBodyIndex :type Integer) (bFromSweep :type Boolean) (SweepResult :type "HitResult Structure (by ref)")))

(event `self.OverlapTrigger.OnComponentEndOverlap`
  (params (OverlappedComponent :type "PrimitiveComponent Object Reference") (OtherActor :type "Actor Object Reference") (OtherComp :type "PrimitiveComponent Object Reference") (OtherBodyIndex :type Integer)))

(event `/Game/Core/UI_Components/BPI_Interact.SetInteractionFocused`
  (params (IsFocused :type Boolean) (InteractingPlayer :type "Character Object Reference"))
  (bind _interactwidget (`self.InteractWidget`))
  (if IsFocused
    (cast `/Game/Core/PlayerBlueprints/BP_Fisherman` InteractingPlayer)
    (set `self.CanInteract` true)
    (`SceneComponent.SetVisibility` _interactwidget true false)
    (if (`KismetSystemLibrary.IsValid` (`self.ActiveMessage`))
      (`SceneComponent.SetVisibility` (`self.InteractWidget`) false false))
    (else
      (cast `/Game/Core/PlayerBlueprints/BP_Fisherman` InteractingPlayer)
      (set `self.CanInteract` false)
      (`SceneComponent.SetVisibility` _interactwidget false false)
      (if (`KismetSystemLibrary.IsValid` (`self.ActiveMessage`))
        (`Widget.RemoveFromParent` (`self.ActiveMessage`))
        (set `self.ActiveMessage` null)))))

(event `self.OnInteract`
  (params (InteractingPlayer :type "Character Object Reference"))
  (if (`self.CanInteract`)
    (cast `/Game/Core/PlayerBlueprints/BP_Fisherman` InteractingPlayer)
    (if (not (`KismetSystemLibrary.IsValid` (`self.ActiveMessage`)))
      (bind _returnvalue (`|CreateWidget` "/Game/Core/UI_Components/OnScreenMessages/Signs/WBP_SignMessage.WBP_SignMessage_C" null (`self.FishToDisplay`)))
      (set `self.ActiveMessage` _returnvalue)
      (`TextBlock.SetText` (`/Game/Core/UI_Components/OnScreenMessages/Signs/WBP_SignMessage.PopupText` _returnvalue) (`KismetTextLibrary.Conv_StringToText` (`KismetTextLibrary.Conv_TextToString` (`self.MessageToShow`))))
      (`UserWidget.AddToViewport` _returnvalue 0)
      (if (`KismetSystemLibrary.IsValid` (`self.ActiveMessage`))
        (`SceneComponent.SetVisibility` (`self.InteractWidget`) false false)))))

(fn `IsInteractable`
  (returns (Interactable :type Boolean))
  (return false))

(fn `UserConstructionScript`)