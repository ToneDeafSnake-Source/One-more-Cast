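; BP_GameMessages is an interactable actor that shows a configurable text message to the player.
; Its overlap trigger toggles an interact prompt for BP_Fisherman, hiding it while a message is active.
; OnInteract creates a single WBP_GameMessage popup from MessageToShow, and leaving the trigger removes it.
; IsInteractable always returns false.
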(event `self.OverlapTrigger.OnComponentBeginOverlap`
  (params (OverlappedComponent :type "PrimitiveComponent Object Reference") (OtherActor :type "Actor Object Reference") (OtherComp :type "PrimitiveComponent Object Reference") (OtherBodyIndex :type Integer) (bFromSweep :type Boolean) (SweepResult :type "HitResult Structure (by ref)"))
  (cast `/Game/Core/PlayerBlueprints/BP_Fisherman` OtherActor)
  (`SceneComponent.SetVisibility` (`self.InteractWidget`) true false)
  (if (`KismetSystemLibrary.IsValid` (`self.ActiveMessage`))
    (`SceneComponent.SetVisibility` (`self.InteractWidget`) false false)))

(event `self.OverlapTrigger.OnComponentEndOverlap`
  (params (OverlappedComponent :type "PrimitiveComponent Object Reference") (OtherActor :type "Actor Object Reference") (OtherComp :type "PrimitiveComponent Object Reference") (OtherBodyIndex :type Integer))
  (cast `/Game/Core/PlayerBlueprints/BP_Fisherman` OtherActor)
  (`SceneComponent.SetVisibility` (`self.InteractWidget`) false false)
  (if (`KismetSystemLibrary.IsValid` (`self.ActiveMessage`))
    (`Widget.RemoveFromParent` (`self.ActiveMessage`))
    (set `self.ActiveMessage` null)))

(event `/Game/Core/UI_Components/BPI_Interact.OnInteract`
  (params (InteractingPlayer :type "Character Object Reference"))
  (cast `/Game/Core/PlayerBlueprints/BP_Fisherman` InteractingPlayer)
  (if (not (`KismetSystemLibrary.IsValid` (`self.ActiveMessage`)))
    (bind _returnvalue (`|CreateWidget` "/Game/Core/UI_Components/OnScreenMessages/WBP_GameMessage.WBP_GameMessage_C"))
    (set `self.ActiveMessage` _returnvalue)
    (`TextBlock.SetText` (`/Game/Core/UI_Components/OnScreenMessages/WBP_GameMessage.PopupText` _returnvalue) (`KismetTextLibrary.Conv_StringToText` (`KismetTextLibrary.Conv_TextToString` (`self.MessageToShow`))))
    (`UserWidget.AddToViewport` _returnvalue 0)
    (if (`KismetSystemLibrary.IsValid` (`self.ActiveMessage`))
      (`SceneComponent.SetVisibility` (`self.InteractWidget`) false false))))

(fn `IsInteractable`
  (returns (Interactable :type Boolean))
  (return false))

(fn `UserConstructionScript`)