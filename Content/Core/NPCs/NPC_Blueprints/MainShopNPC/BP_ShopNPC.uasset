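; BP_ShopNPC is a shop NPC that opens the shop menu when the fisherman player interacts with it.
; An interaction box overlap toggles a prompt widget and gates whether the player can shop.
; On interact, it creates and refreshes WBP_ShopMenu, stores it on the fisherman, and switches to Game and UI input with a cursor.
; SellFish starts disabled, and IsInteractable always returns false.
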(event `self.InteractionBox.OnComponentBeginOverlap`
  (params (OverlappedComponent :type "PrimitiveComponent Object Reference") (OtherActor :type "Actor Object Reference") (OtherComp :type "PrimitiveComponent Object Reference") (OtherBodyIndex :type Integer) (bFromSweep :type Boolean) (SweepResult :type "HitResult Structure (by ref)"))
  (cast `/Game/ThirdPerson/Blueprints/Player_Blueprints/BP_Fisherman` OtherActor)
  (`SceneComponent.SetVisibility` (`self.InteractionWidget`) true false)
  (set `self.CanPlayerShop` true))

(event `self.InteractionBox.OnComponentEndOverlap`
  (params (OverlappedComponent :type "PrimitiveComponent Object Reference") (OtherActor :type "Actor Object Reference") (OtherComp :type "PrimitiveComponent Object Reference") (OtherBodyIndex :type Integer))
  (cast `/Game/ThirdPerson/Blueprints/Player_Blueprints/BP_Fisherman` OtherActor)
  (`SceneComponent.SetVisibility` (`self.InteractionWidget`) false false)
  (set `self.CanPlayerShop` false))

(event `/Game/Core/UI_Components/BPI_Interact.OnInteract`
  (params (InteractingPlayer :type "Character Object Reference"))
  (bind _returnvalue (`GameplayStatics.GetPlayerController` 0))
  (if (`self.CanPlayerShop`)
    (bind _asbp_fisherman (cast `/Game/ThirdPerson/Blueprints/Player_Blueprints/BP_Fisherman` InteractingPlayer))
    (bind _returnvalue_2 (`|CreateWidget` "/Game/Core/UI_Components/Menus/WBP_ShopMenu.WBP_ShopMenu_C" null _asbp_fisherman))
    (`UserWidget.AddToViewport` _returnvalue_2 0)
    (`/Game/Core/UI_Components/Menus/WBP_ShopMenu.RefreshShopMenu` _returnvalue_2)
    (set `/Game/ThirdPerson/Blueprints/Player_Blueprints/BP_Fisherman.ShopMenuWidget` _returnvalue_2 _asbp_fisherman)
    (set `PlayerController.bShowMouseCursor` true _returnvalue)
    (`WidgetBlueprintLibrary.SetInputMode_GameAndUIEx` _returnvalue _returnvalue_2)
    (`Widget.SetIsEnabled` (`/Game/Core/UI_Components/Menus/WBP_ShopMenu.SellFish` _returnvalue_2) false)
    (`Widget.SetKeyboardFocus` _returnvalue_2)))

(fn `IsInteractable`
  (returns (Interactable :type Boolean))
  (return false))

(fn `UserConstructionScript`)