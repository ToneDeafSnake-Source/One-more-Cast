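; Floating trash environment prop that bobs and rocks, animated through its FloatingPivot component.
; On BeginPlay it caches the pivot's relative transform, then starts TL_Floating at a random time so instances move out of phase.
; The timeline's FloatWave drives vertical bob scaled by BobHeight, roll scaled by RockRoll, and a slight pitch.
; Base yaw is preserved, while base roll is overwritten.
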(event `self.ReceiveBeginPlay`
  (`|ExecutionSequence`
    (:`then_0`
      (set `self.BaseLocation` (`SceneComponent.RelativeLocation` (`self.FloatingPivot`))))
    (:`then_1`
      (set `self.BaseRotation` (`SceneComponent.RelativeRotation` (`self.FloatingPivot`))))
    (:`then_2`
      (bind (_direction _floatwave) (`Timeline|TL_Floating` :`NewTime` (`KismetMathLibrary.RandomFloatInRange` 0.0 4.0) :!via `SetNewTime` :!label _label)
        (:`Update`
          (set `self.Float Wave` _floatwave)
          (`SceneComponent.K2_SetRelativeLocation` (`self.FloatingPivot`) (+ (`self.BaseLocation`) (`KismetMathLibrary.MakeVector` 0.0 0.0 (* _floatwave (`self.BobHeight`)))) false false)
          (`SceneComponent.K2_SetRelativeRotation` (`self.FloatingPivot`) (`KismetMathLibrary.MakeRotator` (+ (* _floatwave (`self.RockRoll`)) (`self.Float Wave`)) (+ (.pitch (`self.BaseRotation`)) (`self.Float Wave`)) (.yaw (`self.BaseRotation`))) false false))))
    (:`then_3`
      (goto _label))))

(fn `UserConstructionScript`)