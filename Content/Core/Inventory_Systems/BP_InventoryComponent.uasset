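; Inventory component that holds a fixed-slot array of item data, with fields for fish, junk and treasure.
; On BeginPlay it fills Items with empty structs up to MaxSlots, using HasItem to mark occupied slots.
; AddItem fills the first free slot with quantity one, while other functions set, clear, move or swap slots by index.
; It can grow the slot count and exposes the array for saving and loading.
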(event `self.ReceiveBeginPlay`
  (`self.Initialize_Inventory`))

(fn `AddItem`
  (params (ItemToAdd :type "/Game/Core/Data/Structs/ST_ItemData Structure"))
  (bind (_itemname _basename _quantity _catchdc _sellvalue _itemicon _minweight _maxweight _fishweight _itemid _fishid _quality _islegendaryfish _israrefish _bisfish _hasitem _bisjunk _bistreasure) (break `/Game/Core/Data/Structs/ST_ItemData` ItemToAdd))
  (bind _items (`self.Items`))
  ; Checks for empty slots and adds items to inventory
  (set `self.AddedItem` false)
  (for (_array_element _array_index) _items
    (if (not (`.HasItem_24_B229E3C74CB7715AB075168C6AD1B3E9` (break `/Game/Core/Data/Structs/ST_ItemData` _array_element)))
      (`KismetArrayLibrary.Array_Set` _items _array_index (make `/Game/Core/Data/Structs/ST_ItemData` _itemname "" 1 _catchdc _sellvalue _itemicon _minweight _maxweight _fishweight "None" "None" "NewEnumerator0" _islegendaryfish _israrefish _bisfish true _bisjunk _bistreasure))
      (set `self.AddedItem` true)
      (break))))

(fn `ClearItemAtIndex`
  (params (Index :type Integer))
  (`KismetArrayLibrary.Array_Set` (`self.Items`) Index (make `/Game/Core/Data/Structs/ST_ItemData` "" "" 0 0 0 null)))

(fn `ExpandInventorySlots`
  (params (NewMaxSlots :type Integer))
  (locals (SlotsToAdd :type Integer))
  (if (<= NewMaxSlots (`self.Max Slots`))
    (`KismetSystemLibrary.PrintString` "New max slots is not larger")
    (else
      (bind _output_get (set `self.Max Slots` NewMaxSlots))
      (bind _output_get_2 (set `local.SlotsToAdd` (- _output_get (`KismetArrayLibrary.Array_Length` (`self.Items`)))))
      (for _ (range 1 (+ _output_get_2 1))
        (`KismetArrayLibrary.Array_Add` (`self.Items`) (make `/Game/Core/Data/Structs/ST_ItemData` "" "" 0 0 0 null))))))

(fn `GetItemsForSave`
  (returns (ItemsForSave :type "Array of /Game/Core/Data/Structs/ST_ItemData Structure"))
  (return (`self.Items`)))

(fn `Has room`
  (returns (`Has room` :type Boolean))
  ; Checks if inventory has free slots
  (set `self.FoundEmptySlot` false)
  (for _array_element (`self.Items`)
    (if (not (`.HasItem_24_B229E3C74CB7715AB075168C6AD1B3E9` (break `/Game/Core/Data/Structs/ST_ItemData` _array_element)))
      (set `self.FoundEmptySlot` true)
      (break)))
  (return (`self.FoundEmptySlot`)))

(fn `Initialize_Inventory`
  ; Adds Empty Slots
  (`KismetArrayLibrary.Array_Clear` (`self.Items`))
  (for _ (range (`self.Max Slots`))
    (`KismetArrayLibrary.Array_Add` (`self.Items`) (make `/Game/Core/Data/Structs/ST_ItemData` "" "" 0 0 0 null))))

(fn `LoadItemsForSave`
  (params (LoadedItems :type "Array of /Game/Core/Data/Structs/ST_ItemData Structure"))
  (set `self.Items` LoadedItems))

(fn `MoveOrSwapItem`
  (params (SourceIndex :type Integer) (TargetIndex :type Integer))
  (bind _items (`self.Items`))
  (set `self.CachedSourceIndex` SourceIndex)
  (set `self.CachedTargetIndex` TargetIndex)
  (set `self.TargetItem` (`|GetArrayItem` (`self.Items`) (`self.CachedTargetIndex`)))
  (set `self.SourceItem` (`|GetArrayItem` (`self.Items`) (`self.CachedSourceIndex`)))
  (if (== (`self.CachedSourceIndex`) (`self.CachedTargetIndex`))
    (return)
    (elif (`.HasItem_24_B229E3C74CB7715AB075168C6AD1B3E9` (break `/Game/Core/Data/Structs/ST_ItemData` (`self.SourceItem`)))
      (if (`.HasItem_24_B229E3C74CB7715AB075168C6AD1B3E9` (break `/Game/Core/Data/Structs/ST_ItemData` (`self.TargetItem`)))
        (`KismetArrayLibrary.Array_Set` (`self.Items`) (`self.CachedSourceIndex`) (`self.TargetItem`))
        (`KismetArrayLibrary.Array_Set` (`self.Items`) (`self.CachedTargetIndex`) (`self.SourceItem`))
        (else
          (`KismetArrayLibrary.Array_Set` _items (`self.CachedTargetIndex`) (`self.SourceItem`))
          (`KismetArrayLibrary.Array_Set` _items (`self.CachedSourceIndex`) (make `/Game/Core/Data/Structs/ST_ItemData` "" "" 0 0 0 null)))))))

(fn `RemoveItemAtIndex`
  (params (Index :type Integer))
  ; Removes Items from inventory
  (`self.ClearItemAtIndex` Index))

(fn `SetItemAtIndex`
  (params (Index :type Integer) (ItemData :type "/Game/Core/Data/Structs/ST_ItemData Structure"))
  (`KismetArrayLibrary.Array_Set` (`self.Items`) Index ItemData))