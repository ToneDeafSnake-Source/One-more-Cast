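; BP_FishingSpot is a world actor where a BP_Fisherman casts a line to catch random fish.
; Its InteractionSphere overlap toggles the prompt widget and CanPlayerFish, and leaving cancels any pending catch.
; OnInteract checks inventory room, waits a random bite delay that overwrites MinBiteTime, then adds a FishToCatch entry to player 0's inventory.
; Feedback uses PrintString, and IsInteractable always returns false.
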(event `self.InteractionSphere.OnComponentBeginOverlap`
  (params (OverlappedComponent :type "PrimitiveComponent Object Reference") (OtherActor :type "Actor Object Reference") (OtherComp :type "PrimitiveComponent Object Reference") (OtherBodyIndex :type Integer) (bFromSweep :type Boolean) (SweepResult :type "HitResult Structure (by ref)"))
  ; Determines if player is close enough to the fishing spot
  (cast `/Game/ThirdPerson/Blueprints/Player_Blueprints/BP_Fisherman` OtherActor
    (:`then`
      (`SceneComponent.SetVisibility` (`self.InteractWidget`) true false)
      (set `self.CanPlayerFish` true)
      (`KismetSystemLibrary.PrintString` "Press \"E\" to Fish"))
    (:`CastFailed`
      (`KismetSystemLibrary.PrintString` "Cant fish"))))

(event `self.InteractionSphere.OnComponentEndOverlap`
  (params (OverlappedComponent :type "PrimitiveComponent Object Reference") (OtherActor :type "Actor Object Reference") (OtherComp :type "PrimitiveComponent Object Reference") (OtherBodyIndex :type Integer))
  ; Determines if player is close enough to the fishing spot
  (cast `/Game/ThirdPerson/Blueprints/Player_Blueprints/BP_Fisherman` OtherActor)
  (`SceneComponent.SetVisibility` (`self.InteractWidget`) false false)
  (set `self.CanPlayerFish` false)
  (set `self.IsFishing` false)
  (`KismetSystemLibrary.PrintString` "Left Fishing Spot"))

(event `/Game/Core/BPI_Interact.OnInteract`
  (params (InteractingPlayer :type "Character Object Reference"))
  (bind _fishtocatch (`self.FishToCatch`))
  (bind _returnvalue (`KismetArrayLibrary.Array_Length` _fishtocatch))
  ; Catching Fish
  (bind _asbp_fisherman (cast `/Game/ThirdPerson/Blueprints/Player_Blueprints/BP_Fisherman` InteractingPlayer))
  (bind _has_room (`/Game/Core/Inventory_Systems/BP_InventoryComponent.Has room` (`/Game/ThirdPerson/Blueprints/Player_Blueprints/BP_Fisherman.BP_InventoryComponent` _asbp_fisherman)))
  (if _has_room
    (if (`self.CanPlayerFish`)
      (`SceneComponent.SetVisibility` (`self.InteractWidget`) false false)
      (if (`self.CanPlayerFish`)
        (if (`self.IsFishing`)
          (`KismetSystemLibrary.PrintString` "You are already fishing")
          (else
            (set `self.IsFishing` true)
            (`KismetSystemLibrary.PrintString` "Casting Line...")
            (bind _output_get (set `self.MinBiteTime` (`KismetMathLibrary.RandomFloatInRange` (`self.MinBiteTime`) (`self.MaxBiteTime`))))
            (`KismetSystemLibrary.Delay` _output_get)
            (if (`self.IsFishing`)
              (bind _asbp_fisherman_2 (cast `/Game/ThirdPerson/Blueprints/Player_Blueprints/BP_Fisherman` (`GameplayStatics.GetPlayerCharacter` 0)))
              (bind _output_get_2 (set `self.SelectedFish` (`|GetArrayItem` _fishtocatch (- _returnvalue (`KismetMathLibrary.RandomIntegerInRange` 1 _returnvalue)))))
              (`/Game/Core/Inventory_Systems/BP_InventoryComponent.AddItem` (`/Game/ThirdPerson/Blueprints/Player_Blueprints/BP_Fisherman.BP_InventoryComponent` _asbp_fisherman_2) _output_get_2)
              (`KismetSystemLibrary.PrintString` (`KismetStringLibrary.Concat_StrStr` "You Caught:" (`.ItemNAme_16_9C0A4AFD48B1C72E8CE0A79560B7F663` (break `/Game/Core/Inventory_Systems/ST_ItemData` _output_get_2))))
              (`SceneComponent.SetVisibility` (`self.InteractWidget`) true false)
              (set `self.IsFishing` false)
              (else
                (`KismetSystemLibrary.PrintString` "You left the spot")
                (set `self.IsFishing` false)))))))
    (else
      (`KismetSystemLibrary.PrintString` "inventory full!"))))

(fn `IsInteractable`
  (returns (Interactable :type Boolean))
  (return false))

(fn `UserConstructionScript`)